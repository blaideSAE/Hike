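; CryptexPuzzle is a puzzle actor that builds a cryptex with one ring per character of its Password.
; The construction script spawns CryptexRing child actors, evenly spaced between two scene components placed at Top and Bottom.
; It resizes the Rings array to match, keeping each ring's edited Faces across rebuilds, then applies faces and text styling.
; The event graph is empty, so no solving logic lives here.
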(event EventBeginPlay)

(event Collision|EventActorBeginOverlap
  (params (OtherActor :type Actor%20Object%20Reference)))

(event EventTick
  (params (DeltaSeconds :type Float%20%28single-precision%29)))

(fn ConstructionScript
  (bind _password (Variables|Default|GetPassword))
  (bind _scene (Variables|Default|GetScene))
  (bind _rings (Variables|Default|GetRings))
  (bind _newrings (Variables|Default|GetNewRings))
  (bind _rings_2 (Variables|Default|GetRings))
  (bind _rings_3 (Variables|Default|GetRings))
  (bind _returnvalue (Utilities|Array|Length _rings))
  (bind _returnvalue_2 (Utilities|Array|Length _newrings))
  (bind _returnvalue_3 (Utilities|String|GetCharacterArrayfromString _password))
  (bind _returnvalue_4 (Transformation|GetRelativeTransform _scene))
  (bind (_location _rotation _scale) (Math|Transform|BreakTransform _returnvalue_4))
  (Transformation|SetRelativeLocation (Variables|Default|GetScene) (Math|Vector|MakeVector 0.0 0.0 (Variables|Default|GetTop)) false false)
  (Transformation|SetRelativeLocation (Variables|Default|GetScene1) (Math|Vector|MakeVector 0.0 0.0 (Variables|Default|GetBottom)) false false)
  (Utilities|Array|Clear (Variables|Default|GetNewRings))
  (for (_ _array_index) _returnvalue_3
    (bind _returnvalue_5 (AddComponent|AddChildActorComponent false (Math|Transform|MakeTransform (Math|Vector|Lerp(Vector) (Variables|/Script/Engine.SceneComponent|GetRelativeLocation (Variables|Default|GetScene)) (Variables|/Script/Engine.SceneComponent|GetRelativeLocation (Variables|Default|GetScene1)) (/ (Math|Conversions|ToFloat(Integer) _array_index) (Math|Conversions|ToFloat(Integer) (- (Utilities|Array|Length _returnvalue_3) 1)))) _rotation _scale)))
    (bind _ascryptex_ring (Utilities|Casting|CastToCryptexRing (Variables|/Script/Engine.ChildActorComponent|GetChildActor _returnvalue_5)))
    (Utilities|Array|Add (Variables|Default|GetNewRings) (Utilities|Struct|MakeCryptexRingData _ascryptex_ring)))
  (while (> _returnvalue _returnvalue_2)
    (Utilities|Array|RemoveIndex _rings_3 (Utilities|Array|LastIndex _rings_3)))
  (while (< _returnvalue _returnvalue_2)
    (Utilities|Array|Add :TargetArray (Variables|Default|GetRings)))
  (for (_array_element _array_index_2) (Variables|Default|GetNewRings)
    (Utilities|Array|SetArrayElem _rings_2 _array_index_2 (Utilities|Struct|MakeCryptexRingData (.Ring (Utilities|Struct|BreakCryptexRingData _array_element)) (.Faces (Utilities|Struct|BreakCryptexRingData (Utilities|Array|Get(acopy) _rings_2 _array_index_2)))))
    (Variables|/Game/Blueprints/PuzzleParts/CryptexParts/CryptexRing.CryptexRing_C|SetFaces (.Ring (Utilities|Struct|BreakCryptexRingData _array_element)) (.Faces (Utilities|Struct|BreakCryptexRingData (Utilities|Array|Get(acopy) _rings_2 _array_index_2))))
    (Default|SetUpFaces (.Ring (Utilities|Struct|BreakCryptexRingData (Utilities|Array|Get(acopy) _rings_2 _array_index_2))))
    (Default|SetTextSettings (.Ring (Utilities|Struct|BreakCryptexRingData (Utilities|Array|Get(acopy) _rings_2 _array_index_2))) (Variables|TextSettings|GetTextSize) (Variables|TextSettings|GetTextMaterial) (Variables|TextSettings|GetFont) (Variables|TextSettings|GetTextColor))))