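; Puzzle-part actor that displays a configurable text message through the FirstPersonCharacter, either on overlap or on demand.
; Overlap shows the text if ShowOnOverlap is set, and it either hides after a delay or stays until overlap ends.
; The Trigger event shows it on the cached player character, always with delayed hiding.
; ShowOnlyOnce limits both paths to one display; the actor's own ShowText function is an empty stub.
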(event EventBeginPlay
  (bind _asfirst_person_character (Utilities|Casting|CastToFirstPersonCharacter (Game|GetPlayerCharacter 0)))
  (Variables|Default|SetPlayerChar _asfirst_person_character))

(event Collision|EventActorBeginOverlap
  (params (OtherActor :type Actor%20Object%20Reference))
  (bind _showonlyonce (Variables|Default|GetShowOnlyOnce))
  (if (or (not _showonlyonce) (and _showonlyonce (not (Variables|Default|GethasBeenShown))))
    (if (Variables|Default|GetShowOnOverlap)
      (bind _asfirst_person_character (Utilities|Casting|CastToFirstPersonCharacter OtherActor))
      (Default|ShowText _asfirst_person_character (Variables|Default|GetText%20To%20Show) (not (Variables|Default|GetStayUntilOverlapEnd)) (Variables|Default|GetDelay))
      (Variables|Default|SethasBeenShown true))))

(event EventTick
  (params (DeltaSeconds :type Float%20%28single-precision%29)))

(event Collision|EventActorEndOverlap
  (params (OtherActor :type Actor%20Object%20Reference))
  (if (Variables|Default|GetStayUntilOverlapEnd)
    (bind _asfirst_person_character (Utilities|Casting|CastToFirstPersonCharacter OtherActor))
    (Default|HIdeText _asfirst_person_character)))

(event EventTrigger
  (bind _showonlyonce (Variables|Default|GetShowOnlyOnce))
  (if (or (not _showonlyonce) (and _showonlyonce (not (Variables|Default|GethasBeenShown))))
    (Default|ShowText (Variables|Default|GetPlayerChar) (Variables|Default|GetText%20To%20Show) true (Variables|Default|GetDelay))
    (Variables|Default|SethasBeenShown true)))

(fn ConstructionScript)

(fn ShowText
  (if (Utilities|IsValid (Game|GetPlayerCharacter 0))
    _))