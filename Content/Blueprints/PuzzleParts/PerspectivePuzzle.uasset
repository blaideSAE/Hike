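; Perspective puzzle actor that is solved when a character views it from a set position and angle.
; Each tick it compares the camera world transform of characters overlapping its Capsule against an Arrow component, within location and rotation tolerances.
; The first match sets Solved and calls PuzzleCompleted once.
; The construction script orients the Arrow from the Direction variable to define the required view.
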(event EventTick
  (params (DeltaSeconds :type Float%20%28single-precision%29))
  (bind _arrow (Variables|Default|GetArrow))
  (for _array_element (Collision|GetOverlappingActors (Variables|Default|GetCapsule) "/Script/Engine.Character" :!class /Script/Engine.PrimitiveComponent)
    (bind _ascharacter (Utilities|Casting|CastToCharacter _array_element))
    (if (Math|Boolean|ANDBoolean (Math|Rotator|Equal(Rotator) (Transformation|GetWorldRotation (Actor|GetComponentbyClass _ascharacter "/Script/Engine.CameraComponent")) (Transformation|GetWorldRotation _arrow) (Variables|Default|GetRotation%20Tolerance)) (Math|Vector|Equal(Vector) (Transformation|GetWorldLocation (Actor|GetComponentbyClass _ascharacter "/Script/Engine.CameraComponent")) (Transformation|GetWorldLocation _arrow) (Variables|Default|GetLocation%20Tolerance)) (not (Variables|Default|Get%20Solved)))
      (Variables|Default|Set%20Solved true)
      (CallFunction|PuzzleCompleted))))

(fn ConstructionScript
  (Transformation|SetRelativeRotation (Variables|Default|GetArrow) (Variables|Default|GetDirection) false false))