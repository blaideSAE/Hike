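; Floor tile for a maze puzzle that shifts its cube when a Character first steps on it.
; It registers in the TileMaze's FloorTiles on BeginPlay and calls TileTriggered on the Maze when stepped on.
; Tick moves the cube to TriggeredOffset over about one second.
; OnReset clears the state, and Tick eases the cube back to origin by lerping from its current position.
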(event EventBeginPlay
  (bind _astile_maze (Utilities|Casting|CastToTileMaze (Variables|Default|GetMaze)))
  (Utilities|Array|Add (Variables|/Game/Blueprints/PuzzleParts/TileMaze.TileMaze_C|GetFloorTiles _astile_maze) self))

(event Collision|EventActorBeginOverlap
  (params (OtherActor :type Actor%20Object%20Reference))
  ;[1 1 1] Get Character
  (Utilities|Casting|CastToCharacter OtherActor)
  (if (not (Variables|Default|GetState))
    (Variables|Default|SetState true)
    (Default|TileTriggered (Variables|Default|GetMaze) self)
    (Variables|Default|SetMovePercent 0.0)))

(event EventTick
  (params (DeltaSeconds :type Float%20%28single-precision%29))
  (Variables|Default|SetMovePercent (+ DeltaSeconds (Variables|Default|GetMovePercent)))
  (if (< (Variables|Default|GetMovePercent) 1.0)
    (if (Variables|Default|GetState)
      (Transformation|SetRelativeLocation (Variables|Default|GetCube) (Math|Vector|Lerp(Vector) "0, 0, 0" (Variables|Default|GetTriggeredOffset) (Variables|Default|GetMovePercent)) false false)
      (else
        (Transformation|SetRelativeLocation (Variables|Default|GetCube) (Math|Vector|Lerp(Vector) (Variables|/Script/Engine.SceneComponent|GetRelativeLocation (Variables|Default|GetCube)) "0, 0, 0" (Variables|Default|GetMovePercent)) false false)))))

(fn ConstructionScript)

(fn OnReset
  (Variables|Default|SetState false)
  (Variables|Default|SetMovePercent 0.0))