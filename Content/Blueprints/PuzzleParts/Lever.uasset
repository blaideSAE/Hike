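; Interactable puzzle lever that drives a list of linked toggleable or triggerable objects.
; When interacted with at either end of its travel, it plays a sound, flips its state, triggers its targets, then either matches their state to its own or toggles them.
; Tick animates the cylinder by interpolating between two rotations.
; With Toggle off, the lever swings back automatically without notifying its targets.
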(event EventTick
  (params (DeltaSeconds :type Float%20%28single-precision%29))
  (bind _cylinder (Variables|Default|GetCylinder))
  (if (and (>= (Variables|Default|GetRotation) 0.0) (<= (Variables|Default|GetRotation) 1.0))
    (if (Variables|Default|GetState)
      (bind _output_get (Variables|Default|SetRotation (+ DeltaSeconds (Variables|Default|GetRotation))))
      (Transformation|SetRelativeRotation _cylinder (Math|Rotator|Lerp(Rotator) (Variables|Default|GetOriginalRotation) (Variables|Default|GetswitchedRotation) _output_get true) false false)
      (if (and (not (Variables|Default|GetToggle)) (>= (Variables|Default|GetRotation) 1.0))
        (Variables|Default|SetState false)
        (Variables|Default|SetRotation 0.99))
      (else
        (bind _output_get_2 (Variables|Default|SetRotation (- (Variables|Default|GetRotation) DeltaSeconds)))
        (Transformation|SetRelativeRotation _cylinder (Math|Rotator|Lerp(Rotator) (Variables|Default|GetOriginalRotation) (Variables|Default|GetswitchedRotation) _output_get_2 true) false false)))))

(event EventInteracted
  (bind _self self)
  (bind _toggleablesortriggerables (Variables|Default|GetToggleablesOrTriggerables))
  (if (or (<= (Variables|Default|GetRotation) 0.0) (>= (Variables|Default|GetRotation) 1.0))
    (Audio|PlaySoundatLocation (Variables|Default|GetSoundEffect) (Transformation|GetActorLocation _self) "0, 0, 0" 1.0 1.0 0.0 0 0 _self)
    (bind _output_get (Variables|Default|SetState (not (Variables|Default|GetState))))
    (if _output_get
      (Variables|Default|SetRotation 0.01)
      (else
        (Variables|Default|SetRotation 0.99)))
    (CallFunction|TriggerAllTriggerables _toggleablesortriggerables)
    (if (Variables|Default|GetMatchToggleState)
      (CallFunction|SetAllToggleables _toggleablesortriggerables (Variables|Default|GetState))
      (else
        (CallFunction|ToggleAllToggleables _toggleablesortriggerables)))))

(fn ConstructionScript)