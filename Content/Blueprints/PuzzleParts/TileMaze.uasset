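; TileMaze is a puzzle actor that builds a centred X-by-Y grid of Tile child actors and checks their states.
; The construction script spawns the evenly spaced tiles and stores them in FloorTiles.
; TileTriggered resets every tile on a state mismatch; otherwise it compares all tiles to their targets, though the win branch is empty.
; The Trigger event also resets all tiles.
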(event EventBeginPlay)

(event Collision|EventActorBeginOverlap
  (params (OtherActor :type Actor%20Object%20Reference)))

(event EventTick
  (params (DeltaSeconds :type Float%20%28single-precision%29)))

(event EventTrigger
  (CallFunction|ResetAllTiles))

(fn ConstructionScript
  (bind _x (Variables|Default|GetX))
  (bind _y (Variables|Default|GetY))
  (bind _tile_spacing (Variables|Default|GetTile%20Spacing))
  ;[1 1 1] Creating tiles, Adding them to the array
  (for _index (range 1 _x)
    (for _index_2 (range 1 _y)
      (bind _returnvalue (AddComponent|AddChildActorComponent false (Math|Transform|MakeTransform (Math|Vector|MakeVector (* (- (Math|Conversions|ToFloat(Integer) _index) (/ (Math|Conversions|ToFloat(Integer) (+ _x 1)) 2.0)) _tile_spacing) (* (- (Math|Conversions|ToFloat(Integer) _index_2) (/ (Math|Conversions|ToFloat(Integer) (+ _y 1)) 2.0)) _tile_spacing) 0.0))))
      (bind _astile (Utilities|Casting|CastToTile (Variables|/Script/Engine.ChildActorComponent|GetChildActor _returnvalue)))
      (Utilities|Array|Add (Variables|Default|GetFloorTiles) _astile))))

(fn TileTriggered
  (params (Actor :type Tile%20Object%20Reference))
  (if (Math|Boolean|Equal(Boolean) (Variables|/Game/Blueprints/PuzzleParts/Tile.Tile_C|GetTargetState Actor) (Variables|/Game/Blueprints/PuzzleParts/Tile.Tile_C|GetState Actor))
    (for _array_element (Variables|Default|GetFloorTiles)
      (if (not (Math|Boolean|Equal(Boolean) (Variables|/Game/Blueprints/PuzzleParts/Tile.Tile_C|GetState _array_element) (Variables|/Game/Blueprints/PuzzleParts/Tile.Tile_C|GetTargetState _array_element)))
        (LocalVariables|SetWinFlag false)))
    (if (LocalVariables|GetWinFlag)
      _)
    (else
      (CallFunction|ResetAllTiles))))

(fn ResetAllTiles
  (for _array_element (Variables|Default|GetFloorTiles)
    (bind _astile (Utilities|Casting|CastToTile _array_element))
    (Variables|/Game/Blueprints/PuzzleParts/Tile.Tile_C|SetState _astile false)
    (Default|OnReset _astile)))