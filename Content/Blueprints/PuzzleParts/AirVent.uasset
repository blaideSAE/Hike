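; Puzzle air vent that, while active, lifts characters along its grate's up axis and holds them near the column's center line.
; Each tick it applies curve-scaled upward force within a radius of that line, plus a distance-weighted centering pull and velocity-opposing drag to stabilize overlapping characters.
; Toggle events switch the force and Niagara effect.
; The construction script fits the capsule and effect to MaxHeight and sets grate visibility.
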(event EventBeginPlay
  (Components|Activation|SetActive (Variables|Default|GetNiagara) (Variables|Default|GetActive) true))

(event EventOnToggled
  (Variables|Default|SetActive (not (Variables|Default|GetActive)))
  (Components|Activation|SetActive (Variables|Default|GetNiagara) (Variables|Default|GetActive) true))

(event EventTick
  (params (DeltaSeconds :type Float%20%28single-precision%29))
  (bind _airresistance (Variables|Default|GetAirResistance))
  (bind _grate (Variables|Default|GetGrate))
  (bind _returnvalue (Math|Vector|GetUpVector _grate))
  (bind _returnvalue_2 (* _airresistance -1.0))
  (if (Variables|Default|GetActive)
    (for _array_element (Collision|GetOverlappingActors (Variables|Default|GetCapsule) "/Script/Engine.Character" :!class /Script/Engine.PrimitiveComponent)
      (bind _ascharacter (Utilities|Casting|CastToCharacter _array_element))
      (if (< (Math|Vector|Distance(Vector) (Transformation|GetActorLocation _ascharacter) (Math|Vector|FindClosestPointonLine (Transformation|GetActorLocation _ascharacter) (Transformation|GetWorldLocation (Variables|Default|GetCapsule)) _returnvalue)) (Variables|Default|GetUpforceRadius))
        (Physics|AddForce (Variables|/Script/Engine.Character|GetCharacterMovement _ascharacter) (* _returnvalue (* (Variables|Default|GetForce) (* (Variables|Default|GetUp%20Distance%20Influence) (Math|Curves|GetFloatValue (Variables|Default|GetCurve) (/ (Math|Float|Absolute(Float) (- (.Z (Math|Vector|BreakVector (Transformation|GetWorldLocation _grate))) (.Z (Math|Vector|BreakVector (Transformation|GetActorLocation _ascharacter))))) (Variables|Default|GetMaxHeight))))))))
      (Physics|AddForce (Variables|/Script/Engine.Character|GetCharacterMovement _ascharacter) (+ (* (- (Math|Vector|FindClosestPointonLine (Transformation|GetActorLocation _ascharacter) (Transformation|GetWorldLocation (Variables|Default|GetCapsule)) _returnvalue) (Transformation|GetActorLocation _ascharacter)) (+ (Variables|Default|GetPull%20To%20centerLine) (* (Math|Vector|Distance(Vector) (Transformation|GetActorLocation _ascharacter) (Math|Vector|FindClosestPointonLine (Transformation|GetActorLocation _ascharacter) (Transformation|GetWorldLocation (Variables|Default|GetCapsule)) _returnvalue)) (Variables|Default|GetPull%20Distance%20Influence)))) (Math|Vector|MakeVector (* (.X (Math|Vector|BreakVector (Pawn|Components|CharacterMovement|GetLastUpdateVelocity (Variables|/Script/Engine.Character|GetCharacterMovement _ascharacter)))) _returnvalue_2) (* (.Y (Math|Vector|BreakVector (Pawn|Components|CharacterMovement|GetLastUpdateVelocity (Variables|/Script/Engine.Character|GetCharacterMovement _ascharacter)))) _returnvalue_2) (* (.Z (Math|Vector|BreakVector (Pawn|Components|CharacterMovement|GetLastUpdateVelocity (Variables|/Script/Engine.Character|GetCharacterMovement _ascharacter)))) _returnvalue_2)))))))

(event EventOnToggledMatchState
  (params (State :type Boolean))
  (Variables|Default|SetActive State)
  (Components|Activation|SetActive (Variables|Default|GetNiagara) (Variables|Default|GetActive) true))

(fn ConstructionScript
  (bind _capsule (Variables|Default|GetCapsule))
  (bind _maxheight (Variables|Default|GetMaxHeight))
  (bind _returnvalue (* _maxheight 0.5))
  (Transformation|SetRelativeLocation _capsule (Math|Vector|MakeVector 0.0 0.0 (- _returnvalue 1e+02)) false true)
  (Components|Capsule|SetCapsuleHalfHeight _capsule _returnvalue false)
  (Transformation|SetRelativeScale3D (Variables|Default|GetNiagara) (Math|Vector|MakeVector 0.5 0.5 (/ _maxheight 25.0)))
  (Rendering|SetVisibility (Variables|Default|GetGrate) (Variables|Default|GetShowMesh) false))