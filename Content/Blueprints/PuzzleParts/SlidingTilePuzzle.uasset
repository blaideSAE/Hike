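; Sliding tile puzzle that builds a square grid of SlidingTile child actors with one empty slot and reports completion to its parent class.
; ReloadTiles spawns and textures the tiles, and RandomizeTiles shuffles them Fisher-Yates style, swapping two tiles when inversion parity is odd.
; While Active, Tick periodically reshuffles until the inversion count is nonzero and within InversionLimit.
; CheckWinState compares each tile's grid position to its start position.
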(event EventBeginPlay
  (if (Variables|Default|GetRandomize%20on%20start)
    (CallFunction|RandomizeTiles)
    (Variables|TimerStuff|SetActive true)))

(event EventTick
  (params (DeltaSeconds :type Float%20%28single-precision%29))
  (if (Variables|TimerStuff|GetActive)
    (bind _output_get (Variables|TimerStuff|SetTimer (+ DeltaSeconds (Variables|TimerStuff|GetTimer))))
    (if (> _output_get (Variables|TimerStuff|GetTimeBetweenReScramble))
      (Variables|TimerStuff|SetTimer 0.0)
      (bind _out (CallFunction|SumInversions))
      (if (> _out (Variables|Default|GetInversionLimit))
        (CallFunction|RandomizeTiles :!label _label)
        (elif (== _out 0)
          (goto _label)
          (else
            (Variables|TimerStuff|SetActive false)))))))

(event EventTrigger
  (if (or (Variables|Default|GetresetableAfterCompletion) (not (Variables|Default|GetHasBeenCompleted)))
    (Variables|Default|SetEmptyPosition (Utilities|Struct|MakeVector2Int))
    (CallFunction|ReloadTiles)
    (CallFunction|RandomizeTiles)
    (Variables|TimerStuff|SetActive true)))

(fn ConstructionScript
  (if (Variables|Default|GetAutoRefresh)
    (CallFunction|ReloadTiles)))

(fn GridtoWorld
  (params (GridPosition :type Vector%202%20Int%20Structure))
  (bind (_x _y) (Utilities|Struct|BreakVector2Int GridPosition))
  (return (Math|Transform|TransformLocation (Transformation|GetWorldTransform (Variables|Default|GetDefaultSceneRoot)) (Math|Vector|MakeVector (Utilities|GridtoworldSingleCoordinate _x) (Utilities|GridtoworldSingleCoordinate _y) 0.0))))

(fn RandomizeTiles
  (bind _tilecount (Variables|Default|GetTileCount))
  ;[1 1 1] The Fisher Yates Algorithem
  (LocalVariables|Seti (- (* _tilecount _tilecount) 1))
  (while (> (LocalVariables|Geti) 0)
    (LocalVariables|Setj (Math|Float|Floor (* (LocalVariables|Geti) (Math|Random|RandomFloat))))
    (LocalVariables|Setxi (Math|Integer|%(Integer) (LocalVariables|Geti) (Variables|Default|GetTileCount)))
    (LocalVariables|Setyi (Math|Float|Floor (/ (Math|Conversions|ToFloat(Integer) (LocalVariables|Geti)) (Math|Conversions|ToFloat(Integer) (Variables|Default|GetTileCount)))))
    (LocalVariables|Setxj (Math|Integer|%(Integer) (LocalVariables|Getj) (Variables|Default|GetTileCount)))
    (LocalVariables|Setyj (Math|Float|Floor (/ (Math|Conversions|ToFloat(Integer) (LocalVariables|Getj)) (Math|Conversions|ToFloat(Integer) (Variables|Default|GetTileCount)))))
    (CallFunction|SwapTiles (Utilities|Struct|MakeVector2Int (LocalVariables|Getxi) (LocalVariables|Getyi)) (Utilities|Struct|MakeVector2Int (LocalVariables|Getxj) (LocalVariables|Getyj)))
    (Math|Integer|DecrementInt (LocalVariables|Geti)))
  (bind _solvable (CallFunction|IsSolvable))
  (if (not _solvable)
    (CallFunction|ToggleSolvability)))

(fn SwapTiles
  (params (TileA :type Vector%202%20Int%20Structure) (TileB :type Vector%202%20Int%20Structure))
  (bind (_x _y) (Utilities|Struct|BreakVector2Int TileB))
  (bind (_x_2 _y_2) (Utilities|Struct|BreakVector2Int TileA))
  (bind _sliding_tiles (Variables|Default|GetSliding%20Tiles))
  (bind _tilecount (Variables|Default|GetTileCount))
  (bind (_value _returnvalue) (Utilities|Map|Find _sliding_tiles TileA))
  (bind (_value_2 _returnvalue_2) (Utilities|Map|Find _sliding_tiles TileB))
  (if (Math|Boolean|ANDBoolean _returnvalue _returnvalue_2 (< _x_2 _tilecount) (< _y_2 _tilecount) (< _x _tilecount) (< _y _tilecount))
    (LocalVariables|SetSlidingTileA _value)
    (LocalVariables|SetSlidingTileB _value_2)
    (LocalVariables|SetPositionA TileA)
    (bind _worldposition (CallFunction|GridtoWorld (Variables|/Game/Blueprints/PuzzleParts/SlidingTileParts/SlidingTile.SlidingTile_C|GetPositionInGrid (LocalVariables|GetSlidingTileB))))
    (Default|SetPosition (LocalVariables|GetSlidingTileA) _worldposition)
    (Variables|/Game/Blueprints/PuzzleParts/SlidingTileParts/SlidingTile.SlidingTile_C|SetPositionInGrid (LocalVariables|GetSlidingTileA) (Variables|/Game/Blueprints/PuzzleParts/SlidingTileParts/SlidingTile.SlidingTile_C|GetPositionInGrid (LocalVariables|GetSlidingTileB)))
    (Utilities|Map|Add (Variables|Default|GetSliding%20Tiles) TileB (LocalVariables|GetSlidingTileA))
    (bind _worldposition_2 (CallFunction|GridtoWorld (LocalVariables|GetPositionA)))
    (Default|SetPosition (LocalVariables|GetSlidingTileB) _worldposition_2)
    (Variables|/Game/Blueprints/PuzzleParts/SlidingTileParts/SlidingTile.SlidingTile_C|SetPositionInGrid (LocalVariables|GetSlidingTileB) (LocalVariables|GetPositionA))
    (Utilities|Map|Add (Variables|Default|GetSliding%20Tiles) TileA (LocalVariables|GetSlidingTileB))))

(fn CountInversions
  (params (X :type Integer) (Y :type Integer))
  (LocalVariables|Seti X)
  (LocalVariables|Setj Y))

(fn SumInversions
  (bind _tilecount (Variables|Default|GetTileCount))
  (bind _tiles (LocalVariables|GetTiles))
  (bind _returnvalue (Utilities|Array|Length _tiles))
  (bind _returnvalue_2 (- _tilecount 1))
  (Utilities|Array|Clear (LocalVariables|GetTiles))
  (for _index (range 0 _returnvalue_2)
    (for _index_2 (range 0 _returnvalue_2)
      (if (.ReturnValue (Utilities|Map|Find (Variables|Default|GetSliding%20Tiles) (Utilities|Struct|MakeVector2Int _index _index_2)))
        (Utilities|Array|Add (LocalVariables|GetTiles) (Variables|/Game/Blueprints/PuzzleParts/SlidingTileParts/SlidingTile.SlidingTile_C|GetTileNumber (.Value (Utilities|Map|Find (Variables|Default|GetSliding%20Tiles) (Utilities|Struct|MakeVector2Int _index _index_2))))))))
  (LocalVariables|SetInversions 0)
  (for _index_3 (range 0 _returnvalue)
    (for _index_4 (range (+ _index_3 1) (+ _returnvalue 1))
      (if (> (Utilities|Array|Get(acopy) _tiles _index_3) (Utilities|Array|Get(acopy) _tiles _index_4))
        (Math|Integer|IncrementInt (LocalVariables|GetInversions)))))
  (return (LocalVariables|GetInversions)))

(fn IsSolvable
  (bind _out (CallFunction|SumInversions))
  (return (== (Math|Integer|%(Integer) _out 2) 0) _out))

(fn ReloadTiles
  (bind _tilecount (Variables|Default|GetTileCount))
  (bind _tilecount_2 (Variables|Default|GetTileCount))
  (bind _spacing (Variables|Default|GetSpacing))
  (bind _tilecount_3 (Variables|Default|GetTileCount))
  (bind _returnvalue (- _tilecount_3 1))
  (bind _returnvalue_2 (- _tilecount 1))
  (for _array_element (Actor|GetAllChildActors false)
    (if (Utilities|IsValid _array_element)
      (Actor|DestroyActor _array_element)))
  (Utilities|Map|Clear (Variables|Default|GetSliding%20Tiles))
  (for _index (range 0 _returnvalue_2)
    (for _index_2 (range 0 _returnvalue)
      (if (not (and (== _index_2 0) (== _index 0)))
        (bind _returnvalue_3 (AddComponent|AddChildActorComponent false (Math|Transform|MakeTransform (Math|Vector|MakeVector (* (- (Math|Conversions|ToFloat(Integer) _index) (/ (Math|Conversions|ToFloat(Integer) _returnvalue_2) 2.0)) _spacing) (* (- (Math|Conversions|ToFloat(Integer) _index_2) (/ (Math|Conversions|ToFloat(Integer) _returnvalue) 2.0)) _spacing) 0.0))))
        (bind _assliding_tile (Utilities|Casting|CastToSlidingTile (Variables|/Script/Engine.ChildActorComponent|GetChildActor _returnvalue_3)))
        (Variables|/Game/Blueprints/PuzzleParts/SlidingTileParts/SlidingTile.SlidingTile_C|SetParentPuzzle _assliding_tile self)
        (bind _output_get (Variables|/Game/Blueprints/PuzzleParts/SlidingTileParts/SlidingTile.SlidingTile_C|SetPositionInGrid _assliding_tile (Utilities|Struct|MakeVector2Int _index _index_2)))
        (bind _output_get_2 (Variables|/Game/Blueprints/PuzzleParts/SlidingTileParts/SlidingTile.SlidingTile_C|SetStartPosition _assliding_tile (Utilities|Struct|MakeVector2Int _index _index_2)))
        (Variables|/Game/Blueprints/PuzzleParts/SlidingTileParts/SlidingTile.SlidingTile_C|SetTileNumber _assliding_tile (+ (+ _index_2 1) (* _index (Variables|Default|GetTileCount))))
        (Default|SetSpeed _assliding_tile (Variables|Default|GetMovementSpeed))
        (Default|SetMaterial _assliding_tile (Utilities|Struct|MakeVector2Int _tilecount_2 _tilecount_2) _output_get (Variables|Default|GetTexture))
        (Utilities|Map|Add (Variables|Default|GetSliding%20Tiles) _output_get_2 _assliding_tile)
        (else
          (Variables|Default|SetEmptyPosition (Utilities|Struct|MakeVector2Int _index _index_2)))))))

(fn CheckWinState
  (bind _tilecount (Variables|Default|GetTileCount))
  (bind _tilecount_2 (Variables|Default|GetTileCount))
  (bind _returnvalue (- _tilecount 1))
  (LocalVariables|SetCorrectlyLocatedTileCount 0)
  ;[1 1 1] Looping through every tile
  (for _index (range 0 _returnvalue)
    (for _index_2 (range 0 _returnvalue)
      ;;[1 1 1] Comparing the goal position IE start position with their current positon.
      (if (.ReturnValue (Utilities|Map|Find (Variables|Default|GetSliding%20Tiles) (Utilities|Struct|MakeVector2Int _index _index_2)))
        ;;[1 1 1] If they match, Add to the count.
        (if (and (== (.x (Utilities|Struct|BreakVector2Int (Variables|/Game/Blueprints/PuzzleParts/SlidingTileParts/SlidingTile.SlidingTile_C|GetPositionInGrid (.Value (Utilities|Map|Find (Variables|Default|GetSliding%20Tiles) (Utilities|Struct|MakeVector2Int _index _index_2)))))) (.x (Utilities|Struct|BreakVector2Int (Variables|/Game/Blueprints/PuzzleParts/SlidingTileParts/SlidingTile.SlidingTile_C|GetStartPosition (.Value (Utilities|Map|Find (Variables|Default|GetSliding%20Tiles) (Utilities|Struct|MakeVector2Int _index _index_2))))))) (== (.y (Utilities|Struct|BreakVector2Int (Variables|/Game/Blueprints/PuzzleParts/SlidingTileParts/SlidingTile.SlidingTile_C|GetPositionInGrid (.Value (Utilities|Map|Find (Variables|Default|GetSliding%20Tiles) (Utilities|Struct|MakeVector2Int _index _index_2)))))) (.y (Utilities|Struct|BreakVector2Int (Variables|/Game/Blueprints/PuzzleParts/SlidingTileParts/SlidingTile.SlidingTile_C|GetStartPosition (.Value (Utilities|Map|Find (Variables|Default|GetSliding%20Tiles) (Utilities|Struct|MakeVector2Int _index _index_2))))))))
          (Math|Integer|IncrementInt (LocalVariables|GetCorrectlyLocatedTileCount))))))
  ;[1 1 1] if the count of tiles in the correct place = the ammount of tiles, Then they're all in the correct place. The puzzle is complete.
  (if (>= (LocalVariables|GetCorrectlyLocatedTileCount) (- (* _tilecount_2 _tilecount_2) 1))
    (CallFunction|PuzzleCompleted)))

(fn PuzzleCompleted
  (|CallParentFunction))

(fn CheckSolvability
  (bind (_solvable _inversion_sum) (CallFunction|IsSolvable))
  (if _solvable
    (Development|PrintString (Utilities|String|Append "Solvable, " (Utilities|String|ToString(Integer) _inversion_sum) " inversions."))
    (else
      (Development|PrintString (Utilities|String|Append "Not solvable, " (Utilities|String|ToString(Integer) _inversion_sum) " Inversions.")))))

(fn ToggleSolvability
  (bind _tilecount (Variables|Default|GetTileCount))
  (bind _returnvalue (- _tilecount 1))
  (CallFunction|SumInversions)
  (CallFunction|SwapTiles (Utilities|Struct|MakeVector2Int (- _tilecount 2) _returnvalue) (Utilities|Struct|MakeVector2Int _returnvalue _returnvalue))
  (CallFunction|SumInversions))