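; Cryptex ring puzzle part that shows a set of text faces around a cylinder and advances to the next on each interaction.
; The construction script creates one text label per Faces entry, spaced evenly in a circle using TextOffsetTransform for radius and height.
; Interacted wraps CurrentFace, sets the target yaw and prints the face for debugging.
; Tick turns the cylinder by a fixed, frame-rate-dependent step until it nears that target.
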(event EventBeginPlay)

(event Collision|EventActorBeginOverlap
  (params (OtherActor :type Actor%20Object%20Reference)))

(event EventTick
  (params (DeltaSeconds :type Float%20%28single-precision%29))
  (if (not (Math|Rotator|Equal(Rotator) (Variables|/Script/Engine.SceneComponent|GetRelativeRotation (Variables|Default|GetCylinder)) (Variables|Default|GetNewRotation) 0.2))
    (Transformation|AddRelativeRotation (Variables|Default|GetCylinder) "0,0.180000, 0" false false)))

(event EventInteracted
  (bind _facecount (Variables|Default|GetFaceCount))
  (if (== (Variables|Default|GetCurrentFace) (- _facecount 1))
    (Variables|Default|SetCurrentFace 0)
    (else
      (Variables|Default|SetCurrentFace (+ (Variables|Default|GetCurrentFace) 1))))
  (Variables|Default|SetNewRotation (Math|Rotator|MakeRotator 0.0 0.0 (* 1 (* (/ (Math|Conversions|ToFloat(Integer) (Variables|Default|GetCurrentFace)) (Math|Conversions|ToFloat(Integer) _facecount)) 3.6e+02))))
  (Development|PrintString (Utilities|String|Append (Utilities|String|ToString(Integer) (+ (Variables|Default|GetCurrentFace) 1)) "of" (Utilities|String|ToString(Integer) (Variables|Default|GetFaceCount)) " = " (Utilities|String|ToString(Text) (Utilities|Array|Get(acopy) (Variables|Default|GetFaces) (- (Variables|Default|GetCurrentFace) 0))))))

(fn ConstructionScript
  (bind _text_offset_transform (Variables|Default|GetText%20Offset%20Transform))
  (bind _faces (Variables|Default|GetFaces))
  (bind _relativelocation (Variables|/Script/Engine.SceneComponent|GetRelativeLocation _text_offset_transform))
  (bind _z (Math|Vector|BreakVector _relativelocation))
  (bind _returnvalue (Math|Vector|MakeVector 0.0 0.0 _z))
  (bind _output_get (Variables|Default|SetFaceCount (Utilities|Array|Length _faces)))
  (for (_array_element _array_index) _faces
    (bind _returnvalue_2 (AddComponent|AddTextRenderComponent false (Transformation|GetRelativeTransform _text_offset_transform)))
    (Rendering|Components|TextRender|SetText _returnvalue_2 _array_element)
    (Transformation|SetRelativeLocation _returnvalue_2 (+ (* (Math|Vector|GetForwardVector (Math|Rotator|MakeRotator 0.0 0.0 (* -1 (* (/ (Math|Conversions|ToFloat(Integer) _array_index) (Math|Conversions|ToFloat(Integer) _output_get)) 3.6e+02)))) (Math|Vector|Distance(Vector) _returnvalue _relativelocation)) _returnvalue) false false)
    (Transformation|SetRelativeRotation _returnvalue_2 (Math|Rotator|MakeRotator 0.0 0.0 (* -1 (* (/ (Math|Conversions|ToFloat(Integer) _array_index) (Math|Conversions|ToFloat(Integer) _output_get)) 3.6e+02))) false false)
    (Rendering|Components|TextRender|SetHorizontalAlignment _returnvalue_2 "EHTA_Center")
    (Utilities|Array|Add (Variables|Default|GetLabels) _returnvalue_2)))

(fn SetUpFaces
  (AddComponent|AddStaticMeshComponent false))